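; Paintable canvas actor that reveals an oil-painting rendition of a source image, which can be a scene capture from the player camera.
; Painter-interface actors entering its trigger supply ray hits that move a smoothed brush cursor with adjustable size, hardness and opacity.
; Brush stamps, timed by stroke speed, accumulate in a mask render target.
; HLSL materials turn mask and source into color and normal render targets displayed on the plane.
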(event OnComponentBeginOverlap(TriggerBox)
  (params (OverlappedComponent :type Primitive%20Component%20Object%20Reference) (OtherActor :type Actor%20Object%20Reference) (OtherComp :type Primitive%20Component%20Object%20Reference) (OtherBodyIndex :type Integer) (bFromSweep :type Boolean) (SweepResult :type Hit%20Result%20Structure%20%28by%20ref%29))
  ;[0.15 0.15 0.15 0.5] in / out collision
  (if (Utilities|DoesObjectImplementInterface OtherActor "/Script/Shader.Painter")
    (Class|Painter|SetPaintable(Message) OtherActor self)
    (Variables|Default|SetBrushSize (.X (Math|Vector|BreakVector (Variables|/Script/Engine.SceneComponent|GetRelativeScale3D (Variables|Default|Getbrush)))))))

(event OnComponentEndOverlap(TriggerBox)
  (params (OverlappedComponent :type Primitive%20Component%20Object%20Reference) (OtherActor :type Actor%20Object%20Reference) (OtherComp :type Primitive%20Component%20Object%20Reference) (OtherBodyIndex :type Integer))
  ;[0.15 0.15 0.15 0.5] in / out collision
  (if (Utilities|DoesObjectImplementInterface OtherActor "/Script/Shader.Painter")
    (Class|Painter|ClearPaintable(Message) OtherActor self)
    (Variables|Default|SetisHit false)))

(event Custom|Capture_1
  ;[0 0.09437 0.15] interface
  (CallFunction|InitializeCaptureRT)
  (CallFunction|InitializeCompositeRT)
  (CallFunction|CaptureScenetoRT)
  (CallFunction|CapturedRTtoHLSL))

(event Custom|Initialize%20Brush%20MID
  (bind _brush (Variables|Default|Getbrush))
  (bind _returnvalue (Rendering|Material|GetMaterial _brush 0))
  ;[0.15 0.15 0.15 0.5] initialize brush material
  (Utilities|IsValid (Variables|Default|GetMID_VisualBrush)
    (:Is%20Not%20Valid
      (Utilities|FlowControl|Sequence
        (:then_0
          (bind _returnvalue_2 (Rendering|Material|CreateDynamicMaterialInstance _brush 1 _returnvalue "MID_RealBrush" :!class /Script/Engine.PrimitiveComponent))
          (bind _output_get (Variables|Default|SetMID_ActualBrush _returnvalue_2))
          (Rendering|Material|SetScalarParameterValue _output_get "Opacity" 0.25 :!class /Script/Engine.MaterialInstanceDynamic)
          (Rendering|Material|SetVectorParameterValue :self _output_get :ParameterName "Color" :!class /Script/Engine.MaterialInstanceDynamic)
          (Rendering|Material|SetScalarParameterValue _output_get "Outline" 0.0 :!class /Script/Engine.MaterialInstanceDynamic))
        (:then_1
          (bind _returnvalue_3 (Rendering|Material|CreateDynamicMaterialInstance _brush 0 _returnvalue "MID_BrushCircle" :!class /Script/Engine.PrimitiveComponent))
          (bind _output_get_2 (Variables|Default|SetMID_VisualBrush _returnvalue_3))
          (Rendering|Material|SetScalarParameterValue _output_get_2 "Opacity" (.x (Variables|Default|GetOpacityMinMax)) :!class /Script/Engine.MaterialInstanceDynamic)
          (Rendering|Material|SetMaterial (Variables|Default|Getbrush) 0 _output_get_2))))))

(event Custom|OnBrushParmChanged
  (bind _mid_visualbrush (Variables|Default|GetMID_VisualBrush))
  ;[0.15 0.15 0.15 0.5] Fade Out
  (Utilities|FlowControl|Sequence
    (:then_0
      (bind _newtrack_0 (Timeline|FadeOutTimeline Stop)
        (:Update
          (Rendering|Material|SetScalarParameterValue _mid_visualbrush "Opacity" (Math|Float|Lerp 0.0 (Math|Float|Power (stale _returnvalue) 0.5) _newtrack_0) :!class /Script/Engine.MaterialInstanceDynamic))
        (:Finished
          (Rendering|Material|SetScalarParameterValue _mid_visualbrush "Opacity" 0.0 :!class /Script/Engine.MaterialInstanceDynamic))))
    (:then_1
      (bind _returnvalue (Rendering|Material|GetScalarParameterValue (Variables|Default|GetMID_ActualBrush) "Opacity" :!class /Script/Engine.MaterialInstanceDynamic))
      (Rendering|Material|SetScalarParameterValue (Variables|Default|GetMID_VisualBrush) "Opacity" (Math|Float|Power _returnvalue 0.5) :!class /Script/Engine.MaterialInstanceDynamic)
      (Utilities|FlowControl|RetriggerableDelay 0.5)
      (Timeline|FadeOutTimeline PlayFromStart))))

(event Custom|Initialize%20Composite%20RT
  (bind _canvassize (Variables|Default|GetCanvasSize))
  ;[0.15 0.15 0.15 0.5] Initialize Capture RT
  (Utilities|IsValid (Variables|Default|GetRT_Composite)
    (:Is%20Not%20Valid
      (bind _returnvalue (CanvasRenderTarget2D|CreateCanvasRenderTarget2D "/Script/Engine.CanvasRenderTarget2D" (Math|Float|Truncate (.x _canvassize)) (Math|Float|Truncate (.y _canvassize))))
      (Variables|Default|SetRT_Composite _returnvalue))))

(event Custom|Initialize%20Capture%20RT
  (bind _canvassize (Variables|Default|GetCanvasSize))
  ;[0.15 0.15 0.15 0.5] Initialize Capture RT
  (Utilities|IsValid (Variables|Default|GetRT_SceneCapture)
    (:Is%20Not%20Valid
      (bind _returnvalue (CanvasRenderTarget2D|CreateCanvasRenderTarget2D "/Script/Engine.CanvasRenderTarget2D" (Math|Float|Truncate (.x _canvassize)) (Math|Float|Truncate (.y _canvassize))))
      (bind _output_get (Variables|Default|SetRT_SceneCapture _returnvalue))
      (Rendering|ClearRenderTarget2D _output_get "(R=0.070360,G=0.000000,B=0.004025,A=0.000000)"))))

(event Custom|UpdateSrcTex
  ;[0.15 0.15 0.15 0.5] update source tex
  (bind _returnvalue (Rendering|Material|GetTextureParameterValue (Variables|Default|GetMID_DrawHLSL) "SrcTexture" :!class /Script/Engine.MaterialInstanceDynamic))
  (Variables|Default|Setout_SrcTex _returnvalue))

(event Custom|Capture%20Scene%20to%20RT
  (bind _returnvalue (Viewport|GetViewportSize))
  (bind _returnvalue_2 (Transformation|GetActorTransform))
  (bind _returnvalue_3 (Game|GetPlayerCameraManager 0))
  (bind _canvassize (Variables|Default|GetCanvasSize))
  (bind _returnvalue_4 (Camera|GetFOVAngle _returnvalue_3))
  ;[0.15 0.15 0.15 0.5] Capture Scene
  (bind _returnvalue_5 (AddComponent|AddSceneCaptureComponent2D false (Math|Transform|MakeTransform (Math|Transform|InverseTransformLocation _returnvalue_2 (Camera|GetCameraLocation _returnvalue_3)) (Math|Transform|InverseTransformRotation _returnvalue_2 (Camera|GetCameraRotation _returnvalue_3)))))
  (Variables|/Script/Engine.SceneCaptureComponent2D|SetFOVAngle _returnvalue_5 (Math|Float|SelectFloat _returnvalue_4 (Utilities|HfovtoVfov _returnvalue_4) (< (/ (.x _canvassize) (.y _canvassize)) (/ (.x _returnvalue) (.y _returnvalue)))))
  (Variables|/Script/Engine.SceneCaptureComponent2D|SetTextureTarget _returnvalue_5 (Variables|Default|GetRT_SceneCapture))
  (Variables|/Script/Engine.SceneCaptureComponent|SetHiddenActors _returnvalue_5 (Variables|Default|GetCaptureExclusion))
  (Rendering|SceneCapture|CaptureScene _returnvalue_5 :!class /Script/Engine.SceneCaptureComponent2D))

(event Custom|Captured%20RT%20to%20HLSL
  (bind _rt_composite (Variables|Default|GetRT_Composite))
  ;[0.15 0.15 0.15 0.5] RT to HLSL
  (Utilities|FlowControl|Sequence
    (:then_0
      (bind _returnvalue (Rendering|Material|CreateDynamicMaterialInstance "/Game/Shaders/OilPainting/M_SceneCapture.M_SceneCapture" "MID_SceneCapture" "None" :!class /Script/Engine.KismetMaterialLibrary))
      (bind _output_get (Variables|Default|SetMID_SceneCapture _returnvalue))
      (Rendering|Material|SetTextureParameterValue _output_get "Capture" (Variables|Default|GetRT_SceneCapture))
      (Rendering|Material|SetVectorParameterValue _output_get "BackgroundColor" (Class|KismetMathLibrary|HSVtoRGB (Math|Random|RandomFloatinRange 0.0 3.6e+02) 0.924 0.046665 1.0) :!class /Script/Engine.MaterialInstanceDynamic)
      (CallFunction|DrawtoCanvas "(X=0.500000,Y=0.500000)" (Variables|Default|GetCanvasSize) (Variables|Default|GetRT_Composite) (Variables|Default|GetMID_SceneCapture) false))
    (:then_1
      (bind _returnvalue_2 (Rendering|Material|CreateDynamicMaterialInstance (Variables|Default|GetDebugPlane) 0 "/Game/Shaders/OilPainting/MD_Capture.MD_Capture" "None" :!class /Script/Engine.PrimitiveComponent))
      (Rendering|Material|SetTextureParameterValue _returnvalue_2 "Param" (Variables|Default|GetRT_Composite))
      (Rendering|Material|SetMaterial (Variables|Default|GetDebugPlane) 0 _returnvalue_2))
    (:then_2
      (Rendering|Material|SetTextureParameterValue (Variables|Default|GetMID_DrawHLSL) "SrcTexture" _rt_composite)
      (Utilities|IsValid _rt_composite
        (:Is%20Valid
          (Development|PrintString "Captured"))))))

(event Custom|Initialize%20Normal%20MID
  ;[0.15 0.15 0.15 0.5] Normal MID RT
  (Utilities|IsValid (Variables|Default|GetMID_NormalHLSL)
    (:Is%20Not%20Valid
      (bind _returnvalue (Rendering|Material|CreateDynamicMaterialInstance "/Game/Shaders/OilPainting/M_Normal_HLSL.M_Normal_HLSL" "MID_Normal" "None" :!class /Script/Engine.KismetMaterialLibrary))
      (Variables|Default|SetMID_NormalHLSL _returnvalue))))

(event Custom|Initialize%20Normal%20RT
  (bind _canvassize (Variables|Default|GetCanvasSize))
  ;[0.15 0.15 0.15 0.5] Normal MID RT
  (Utilities|IsValid (Variables|Default|GetRT_Normal%20Result)
    (:Is%20Not%20Valid
      (bind _returnvalue (CanvasRenderTarget2D|CreateCanvasRenderTarget2D "/Script/Engine.CanvasRenderTarget2D" (Math|Float|Truncate (.x _canvassize)) (Math|Float|Truncate (.y _canvassize))))
      (Variables|Default|SetRT_Normal%20Result _returnvalue))))

(event Custom|Initialize%20Mask%20RT
  (bind _plane (Variables|Default|GetPlane))
  (bind _relativescale3d (Variables|/Script/Engine.SceneComponent|GetRelativeScale3D _plane))
  (bind (_x _y) (Math|Vector|BreakVector _relativescale3d))
  ;[0.15 0.15 0.15 0.5] Initialize Mask RT
  (Utilities|IsValid (Variables|Default|GetRT_CanvasMask)
    (:Is%20Not%20Valid
      (bind _output_get (Variables|Default|SetScaleToPixel (/ 1024.0 (Math|Float|Max(Float) _x _y))))
      (bind _output_get_2 (Variables|Default|SetCanvasSize (* (Math|Vector2D|MakeVector2D _x _y) _output_get)))
      (bind _returnvalue (CanvasRenderTarget2D|CreateCanvasRenderTarget2D "/Script/Engine.CanvasRenderTarget2D" (Math|Float|Truncate (.x _output_get_2)) (Math|Float|Truncate (.y _output_get_2))))
      (bind _output_get_3 (Variables|Default|SetRT_CanvasMask _returnvalue))
      (Rendering|ClearRenderTarget2D _output_get_3 "(R=1.000000,G=1.000000,B=1.000000,A=1.000000)"))))

(event Custom|Initialize%20MID%20Draw%20HLSL
  (bind _canvassize (Variables|Default|GetCanvasSize))
  (bind _returnvalue (|((a/b)*c) _canvassize 1024.0 1.92e+03))
  ;[0.15 0.15 0.15 0.5] Initialize MID Canvas
  (Utilities|IsValid (Variables|Default|GetMID_DrawHLSL)
    (:Is%20Not%20Valid
      (bind _returnvalue_2 (Rendering|Material|CreateDynamicMaterialInstance (Variables|Default|GetMI_Plane_Original) "MID_DrawStrokes" "None" :!class /Script/Engine.KismetMaterialLibrary))
      (bind _output_get (Variables|Default|SetMID_DrawHLSL _returnvalue_2))
      (Rendering|Material|SetTextureParameterValue _output_get "MaskTexture" (Variables|Default|GetRT_CanvasMask))
      (Rendering|Material|SetVectorParameterValue _output_get "Resolution" (Math|Color|MakeColor (.x _returnvalue) (.y _returnvalue) 0.0) :!class /Script/Engine.MaterialInstanceDynamic)
      (CallFunction|UpdateSrcTex))))

(event Custom|Initialize%20MID%20CanvasRender
  ;[0.15 0.15 0.15 0.5] Initialize Final MID
  (Utilities|IsValid (Variables|Default|GetMID_CanvasRenderer)
    (:Is%20Not%20Valid
      (bind _returnvalue (Rendering|Material|CreateDynamicMaterialInstance "/Game/Shaders/OilPainting/MI_CanvasRender_Painting.MI_CanvasRender_Painting" "MID_CanvasRender" "None" :!class /Script/Engine.KismetMaterialLibrary))
      (bind _output_get (Variables|Default|SetMID_CanvasRenderer _returnvalue))
      (Rendering|Material|SetTextureParameterValue _output_get "BaseColor" (Variables|Default|GetRT_HLSL%20Result))
      (Rendering|Material|SetTextureParameterValue _output_get "Normal" (Variables|Default|GetRT_Normal%20Result))
      (Rendering|Material|SetMaterial (Variables|Default|GetPlane) 0 _output_get))))

(event Custom|Sync%20BrushPos
  (bind _brush (Variables|Default|Getbrush))
  ;[0.15 0.15 0.15 0.5] sync brush position
  (if (Variables|Default|GetisHit)
    (Utilities|FlowControl|Sequence
      (:then_0
        (Utilities|FlowControl|DoOnce false :!label _label))
      (:then_1
        (Transformation|SetRelativeLocation _brush (Math|Interpolation|VInterpTo (Variables|/Script/Engine.SceneComponent|GetRelativeLocation _brush) (Math|Transform|InverseTransformLocation (Transformation|GetActorTransform) (|(((normalize(a))*b)+c) (Math|Vector|GetUpVector (Variables|Default|GetPlane)) 1.0 (Variables|Default|GetHitLocation))) (Utilities|Time|GetWorldDeltaSeconds) 1e+01) false false)))
    (else
      (goto _label Reset))))

(event Custom|Initialize%20RT%20HLSL%20Result
  (bind _canvassize (Variables|Default|GetCanvasSize))
  ;[0.15 0.15 0.15 0.5] Initialize HLSL Result RT
  (Utilities|IsValid (Variables|Default|GetRT_HLSL%20Result)
    (:Is%20Not%20Valid
      (bind _returnvalue (CanvasRenderTarget2D|CreateCanvasRenderTarget2D "/Script/Engine.CanvasRenderTarget2D" (Math|Float|Truncate (.x _canvassize)) (Math|Float|Truncate (.y _canvassize))))
      (bind _output_get (Variables|Default|SetRT_HLSL%20Result _returnvalue))
      ;;[0.15 0.15 0.15 0.5] Initialize draw plain canvas
      (CallFunction|DrawtoCanvas "(X=0.500000,Y=0.500000)" (Variables|Default|GetCanvasSize) _output_get (Variables|Default|GetMID_DrawHLSL) true)
      (Rendering|Material|SetTextureParameterValue (Variables|Default|GetMID_NormalHLSL) "BaseColor" _output_get))))

(event Custom|Deactivate%20Brush
  ;[0.15 0.15 0.15 0.5] brush visibility
  (Components|Activation|SetActive (Variables|Default|Getbrush) false false)
  (Rendering|SetVisibility (Variables|Default|Getbrush) false false))

(event Custom|Activate%20Brush
  ;[0.15 0.15 0.15 0.5] brush visibility
  (Components|Activation|SetActive (Variables|Default|Getbrush) true false)
  (Rendering|SetVisibility (Variables|Default|Getbrush) true false))

(event Custom|Do%20Paint
  (bind _plane (Variables|Default|GetPlane))
  (bind _mid_canvasrenderer (Variables|Default|GetMID_CanvasRenderer))
  (bind _mid_drawhlsl (Variables|Default|GetMID_DrawHLSL))
  (bind _canvassize (Variables|Default|GetCanvasSize))
  ;[0.15 0.15 0.15 0.5] Real Paint
  (Utilities|FlowControl|Sequence
    (:then_0
      (CallFunction|DrawtoCanvas (Variables|Default|GetHitUV) (Math|Conversions|ToVector2D(Vector) (* (Variables|Default|GetBrushSize) (Variables|Default|GetScaleToPixel))) (Variables|Default|GetRT_CanvasMask) (Variables|Default|GetMID_ActualBrush) false)
      (CallFunction|DrawtoCanvas "(X=0.500000,Y=0.500000)" _canvassize (Variables|Default|GetRT_HLSL%20Result) _mid_drawhlsl true "(R=0.000000,G=0.000000,B=0.000000,A=1.000000)")
      (CallFunction|DrawtoCanvas "(X=0.500000,Y=0.500000)" (Variables|Default|GetCanvasSize) (Variables|Default|GetRT_Normal%20Result) (Variables|Default|GetMID_NormalHLSL) true)
      (CallFunction|DrawtoCanvas "(X=0.500000,Y=0.500000)" _canvassize "/Game/Shaders/OilPainting/RTD_Preview.RTD_Preview" _mid_drawhlsl true "(R=0.000000,G=0.000000,B=0.000000,A=1.000000)"))
    (:then_1
      (if (!= (Rendering|Material|GetMaterial _plane 0) _mid_canvasrenderer)
        (Rendering|Material|SetMaterial _plane 0 _mid_canvasrenderer)))))

(event Custom|OnRayHit_1
  (params (HitPosition :type Vector%20%28by%20ref%29) (HitUV :type Vector%202D%20Structure%20%28by%20ref%29))
  ;[0 0.09437 0.15] interface
  (Variables|Default|SetisHit true)
  (Variables|Default|SetHitUV HitUV)
  (bind _output_get (Variables|Default|SetHitLocation HitPosition))
  (Variables|Default|SetHitSpd (Math|Vector|Distance(Vector) HitPosition (Variables|Default|GetHitLocation_Prev)))
  (Variables|Default|SetHitLocation_Prev _output_get)
  (CallFunction|InitializeRTHLSLResult)
  (CallFunction|InitializeMIDCanvasRender)
  (CallFunction|UpdateRTSrcTex))

(event EventBeginPlay
  (bind _plane (Variables|Default|GetPlane))
  (bind _captureexclusion (Variables|Default|GetCaptureExclusion))
  (Utilities|FlowControl|Sequence
    (:then_0
      ;[0.15 0.15 0.15 0.5] Initialize to plain canvas
      (Variables|Default|SetMI_Plane_Original (Rendering|Material|GetMaterial _plane 0))
      (Rendering|Material|SetMaterial _plane 0 "/Game/Shaders/OilPainting/MI_CanvasRender_Plain.MI_CanvasRender_Plain"))
    (:then_1
      ;[0.15 0.15 0.15 0.5] Initialize Brush Circle Rotation
      (Transformation|SetRelativeRotation (Variables|Default|Getbrush) (Variables|/Script/Engine.SceneComponent|GetRelativeRotation (Variables|Default|GetPlane)) false false))
    (:then_2
      (CallFunction|DeactivateBrush))
    (:then_3
      ;[0.15 0.15 0.15 0.5] to be exclude when capture
      (for _array_element (Variables|Default|GetTags%20To%20Be%20Excluded)
        (bind _outactors (Actor|GetAllActorswithTag _array_element))
        (Utilities|Array|AppendArray _captureexclusion _outactors))
      (Utilities|Array|Add _captureexclusion (Game|GetPlayerCharacter 0)))
    (:then_4
      (CallFunction|InitializeBrushMID)
      (CallFunction|InitializeMaskRT)
      (CallFunction|InitializeMIDDrawHLSL)
      (CallFunction|InitializeNormalMID)
      (CallFunction|InitializeNormalRT)
      (CallFunction|InitializeRTHLSLResult)
      (CallFunction|InitializeMIDCanvasRender))))

(event EventSetBrushSize
  (params (SizeOffset :type Float%20%28single-precision%29))
  ;[0 0.09437 0.15] interface
  (CallFunction|OnBrushParmChanged)
  (bind _output_get (Variables|Default|SetBrushSize (Math|Float|Clamp(Float) (+ (|((a/(abs(a)))*b) SizeOffset 0.01) (.X (Math|Vector|BreakVector (Variables|/Script/Engine.SceneComponent|GetRelativeScale3D (Variables|Default|Getbrush))))) 0.05 0.5)))
  (Transformation|SetRelativeScale3D (Variables|Default|Getbrush) (Math|Conversions|ToVector(Float) _output_get)))

(event EventTick
  (params (DeltaSeconds :type Float%20%28single-precision%29))
  (bind _ishit (Variables|Default|GetisHit))
  (bind _hitspd (Variables|Default|GetHitSpd))
  (bind _brush (Variables|Default|Getbrush))
  (bind _returnvalue (Components|Activation|IsActive _brush))
  (bind _returnvalue_2 (/ _hitspd 3.0))
  (bind _returnvalue_3 (Math|Float|Clamp(Float) _returnvalue_2))
  (bind _returnvalue_4 (Math|Float|Lerp 0.2 0.0 _returnvalue_3))
  (Utilities|FlowControl|Sequence
    (:then_0
      (if (and (not _returnvalue) _ishit)
        (CallFunction|ActivateBrush)))
    (:then_1
      (CallFunction|SyncBrushPos))
    (:then_2
      (if (and _returnvalue (not _ishit))
        (CallFunction|DeactivateBrush)))
    (:then_3
      (Utilities|FlowControl|Sequence
        (:then_0
          (if (Variables|Default|GetbIsPainting)
            (Variables|Default|SetTimeAccumulator%20 (+ (Variables|Default|GetTimeAccumulator%20) (Utilities|Time|GetWorldDeltaSeconds)))
            (if (>= (+ (Variables|Default|GetTimeAccumulator%20) (Utilities|Time|GetWorldDeltaSeconds)) _returnvalue_4)
              (CallFunction|DoPaint)
              (Variables|Default|SetTimeAccumulator%20 (- (Variables|Default|GetTimeAccumulator%20) _returnvalue_4)))))))))

(event EventOnRayExit
  ;[0 0.09437 0.15] interface
  (Variables|Default|SetisHit false))

(event EventSetBrushOpacity
  (params (OpacityOffset :type Float%20%28single-precision%29))
  (bind _opacityminmax (Variables|Default|GetOpacityMinMax))
  (bind _mid_actualbrush (Variables|Default|GetMID_ActualBrush))
  ;[0 0.09437 0.15] interface
  (CallFunction|OnBrushParmChanged)
  (bind _returnvalue (Rendering|Material|GetScalarParameterValue _mid_actualbrush "Opacity" :!class /Script/Engine.MaterialInstanceDynamic))
  (Rendering|Material|SetScalarParameterValue _mid_actualbrush "Opacity" (Math|Float|Clamp(Float) (+ _returnvalue (|((a/(abs(a)))*b) OpacityOffset 0.05)) (.x _opacityminmax) (.y _opacityminmax)) :!class /Script/Engine.MaterialInstanceDynamic))

(event EventPaint
  ;[0 0.09437 0.15] interface
  (Variables|Default|SetbIsPainting true))

(event EventSetBrushHardness
  (params (HardnessOffset :type Float%20%28single-precision%29))
  (bind _mid_visualbrush (Variables|Default|GetMID_VisualBrush))
  ;[0 0.09437 0.15] interface
  (CallFunction|OnBrushParmChanged)
  (bind _returnvalue (Rendering|Material|GetScalarParameterValue _mid_visualbrush "Hardness" :!class /Script/Engine.MaterialInstanceDynamic))
  (Rendering|Material|SetScalarParameterValue _mid_visualbrush "Hardness" (Math|Float|Clamp(Float) (+ _returnvalue (|((a/(abs(a)))*b) HardnessOffset -0.05))) :!class /Script/Engine.MaterialInstanceDynamic))

(event EventPaintEnd
  ;[0 0.09437 0.15] interface
  (Variables|Default|SetbIsPainting false)
  (Variables|Default|SetTimeAccumulator%20 0.0))

(fn ConstructionScript)

(fn DrawtoCanvas
  (params (Draw%20UV%20%28Center%29 :type Vector%202D%20Structure) (Brush%20Size :type Vector%202D%20Structure) (Render%20Target :type Texture%20Render%20Target%202D%20Object%20Reference) (Brush%20Mat :type Material%20Interface%20Object%20Reference) (Clear%20RT%20first? :type Boolean) (Clear%20Color :type Linear%20Color%20Structure))
  (if Clear%20RT%20first?
    (Rendering|ClearRenderTarget2D Render%20Target Clear%20Color))
  (bind (_canvas _size _context) (Rendering|BeginDrawCanvastoRenderTarget Render%20Target))
  (Canvas|DrawMaterial :self _canvas :RenderMaterial Brush%20Mat :ScreenPosition (|(a-(b/2)) (* _size Draw%20UV%20%28Center%29) Brush%20Size) :ScreenSize Brush%20Size :CoordinateSize "(X=1.000000,Y=1.000000)" :PivotPoint "(X=0.500000,Y=0.500000)")
  (Rendering|EndDrawCanvastoRenderTarget _context))

(fn Capture
  (bind _out_srctex (Variables|Default|Getout_SrcTex))
  (bind _returnvalue (Utilities|IsValid _out_srctex))
  (CallFunction|InitializeCaptureRT)
  (CallFunction|InitializeCompositeRT)
  (CallFunction|CaptureScenetoRT)
  (CallFunction|CapturedRTtoHLSL)
  (CallFunction|InitializeRTHLSLResult)
  (CallFunction|InitializeMIDCanvasRender)
  (CallFunction|UpdateSrcTex)
  (if _returnvalue
    (return _out_srctex _returnvalue)))

(fn OnRayHit
  (params (HitPosition :type Vector%20%28by%20ref%29 :default "0, 0, 0") (HitUV :type Vector%202D%20Structure%20%28by%20ref%29))
  (Variables|Default|SetisHit true)
  (Variables|Default|SetHitUV HitUV)
  (bind _output_get (Variables|Default|SetHitLocation HitPosition))
  (Variables|Default|SetHitSpd (Math|Vector|Distance(Vector) HitPosition (Variables|Default|GetHitLocation_Prev)))
  (Variables|Default|SetHitLocation_Prev _output_get)
  (CallFunction|InitializeRTHLSLResult)
  (CallFunction|InitializeMIDCanvasRender)
  (return (Variables|Default|Getout_SrcTex)))