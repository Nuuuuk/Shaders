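; Custom PCG Blueprint node, titled RotateVector, that rotates each point's vector attribute "V" by that point's rotation.
; Execution converts every spatial input to point data, runs the point loop, carries over the target actor and returns the collected results.
; The loop body writes the rotated vector back to the hard-coded attribute.
; An unconnected branch that rebuilds point rotation from its up vector never runs.
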(fn ExecutewithContext
  (params (InContext :type PCG%20Context%20Structure%20%28by%20ref%29) (Input :type PCG%20Data%20Collection%20Structure%20%28by%20ref%29))
  (bind _returnvalue (Class|PCGDataFunctionLibrary|GetInputs Input))
  (for _array_element _returnvalue
    (bind _aspcgspatial_data (Utilities|Casting|CastToPCGSpatialData (.Data (Utilities|Struct|BreakPCGTaggedData _array_element))))
    (bind _outdata (PCG|FlowControl|PointLoop InContext (SpatialData|ToPointDatawithContext _aspcgspatial_data InContext) 0))
    (Variables|/Script/PCG.PCGSpatialData|SetTargetActor _outdata (Variables|/Script/PCG.PCGSpatialData|GetTargetActor _aspcgspatial_data))
    (Utilities|Array|Add (LocalVariables|GetTaggedDatas) (Utilities|Struct|MakePCGTaggedData _outdata 0 "None")))
  (return (Utilities|Struct|MakePCGDataCollection (LocalVariables|GetTaggedDatas))))

(fn PointLoopBody
  (params (InContext :type PCG%20Context%20Structure%20%28by%20ref%29) (InData :type PCG%20Point%20Data%20Object%20Reference) (InPoint :type PCG%20Point%20Structure%20%28by%20ref%29) (OutMetadata :type PCG%20Metadata%20Object%20Reference) (Iteration :type Integer64))
  (bind _returnvalue (PCG|Metadata|GetVectorAttribute InPoint OutMetadata "V"))
  (PCG|Metadata|SetVectorAttribute InPoint OutMetadata "V" (Math|Vector|RotateVector _returnvalue (.Rotation (Math|Transform|BreakTransform (.Transform (Utilities|Struct|BreakPCGPoint InPoint))))))
  (return InPoint true))

(fn NodeTitleOverride
  (return "RotateVector"))